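; Game mode Blueprint that plays sound feedback for gameplay events in what appears to be an element-merging game.
; On BeginPlay it binds handlers to eight gameplay delegates.
; Lift, move, merge, skill cast and target put each play their own 2D sound.
; The start button, item purchase and game over handlers are empty, and the Blueprint holds no other logic.
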(event Custom|OnElementLiftedDelegate_事件
  (Audio|PlaySound2D "/Engine/VREditor/Sounds/UI/Object_PickUp.Object_PickUp" 1.0 1.0 0.0 0 0))

(event Custom|OnMoveMadeDelegate_事件
  (params (MergedElement :type B%20Element%20Object%20Reference))
  (Audio|PlaySound2D "/Engine/VREditor/Sounds/UI/Object_Snaps_To_Another_Actor.Object_Snaps_To_Another_Actor" 1.0 1.0 0.0 0 0))

(event Custom|OnMergeMadeDelegate_事件
  (params (MergedElement :type B%20Element%20Object%20Reference))
  (Audio|PlaySound2D "/Engine/VREditor/Sounds/UI/Object_Snaps_To_Grid.Object_Snaps_To_Grid" 1.0 1.0 0.0 0 0))

(event Custom|OnSkillCastedDelegate_事件
  (Audio|PlaySound2D "/Engine/VREditor/Sounds/UI/Enter_Play.Enter_Play" 1.0 1.0 0.0 0 0))

(event Custom|OnTargetPutDelegate_事件
  (Audio|PlaySound2D "/Engine/EditorSounds/GamePreview/EjectFromPlayer.EjectFromPlayer" 1.0 1.0 0.0 0 0))

(event Custom|OnItemBoughtDelegate_事件)

(event Custom|OnStartButtonClickedDelegate_事件)

(event Custom|OnGameOverDelegate_事件)

(event EventBeginPlay
  (EventDispatchers|AssignOnElementLiftedDelegate (delegate Custom|OnElementLiftedDelegate_事件))
  (EventDispatchers|AssignOnMoveMadeDelegate (delegate Custom|OnMoveMadeDelegate_事件))
  (EventDispatchers|AssignOnMergeMadeDelegate (delegate Custom|OnMergeMadeDelegate_事件))
  (EventDispatchers|AssignOnSkillCastedDelegate (delegate Custom|OnSkillCastedDelegate_事件))
  (EventDispatchers|AssignOnTargetPutDelegate (delegate Custom|OnTargetPutDelegate_事件))
  (EventDispatchers|AssignOnItemBoughtDelegate (delegate Custom|OnItemBoughtDelegate_事件))
  (EventDispatchers|AssignOnStartButtonClickedDelegate (delegate Custom|OnStartButtonClickedDelegate_事件))
  (EventDispatchers|AssignOnGameOverDelegate (delegate Custom|OnGameOverDelegate_事件)))

(event EventTick
  (params (DeltaSeconds :type Float%20%28single-precision%29)))

(fn ConstructionScript)