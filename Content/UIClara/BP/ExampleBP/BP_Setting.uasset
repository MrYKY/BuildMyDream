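; BP_Setting is an example actor that demonstrates a settings UI by applying its controls to three display character meshes.
; BeginPlay fills a description panel widget and puts one shared dynamic material instance on all three meshes.
; Sphere overlap has BP_Character show or cancel the settings widget, and entry binds its control events.
; These drive mesh scale, body color, looping animation, emissive glow and per-mesh visibility.
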(event OnComponentBeginOverlap(Sphere)
  (params (OverlappedComponent :type Primitive%20Component%20Object%20Reference) (OtherActor :type Actor%20Object%20Reference) (OtherComp :type Primitive%20Component%20Object%20Reference) (OtherBodyIndex :type Integer) (bFromSweep :type Boolean) (SweepResult :type Hit%20Result%20Structure%20%28by%20ref%29))
  ;[1 1 1] Overlab Event for Adding Widget to Viewport
  (bind _asbp_character (Utilities|Casting|CastToBP_Character OtherActor))
  (Default|SettingUI _asbp_character)
  (Variables|Default|SetSettingWidget (Variables|/Game/UIClara/BP/BP_Character.BP_Character_C|GetSettingWidget _asbp_character))
  (EventDispatchers|BindEventtoOnValueChanged (Variables|/Game/UIClara/BP/Widget/Widget_Setting.Widget_Setting_C|GetSliderBar (Variables|Default|GetSettingWidget)) (delegate Custom|SlideBar))
  (EventDispatchers|BindEventtoOnCheckStateChanged (Variables|/Game/UIClara/BP/Widget/Widget_Setting.Widget_Setting_C|GetRadioButton1 (Variables|Default|GetSettingWidget)) (delegate Custom|RadioButton1))
  (EventDispatchers|BindEventtoOnCheckStateChanged (Variables|/Game/UIClara/BP/Widget/Widget_Setting.Widget_Setting_C|GetRadioButton2 (Variables|Default|GetSettingWidget)) (delegate Custom|RadioButton2))
  (EventDispatchers|BindEventtoOnSelectionChanged (Variables|/Game/UIClara/BP/Widget/Widget_Setting.Widget_Setting_C|GetDropDownBox (Variables|Default|GetSettingWidget)) (delegate Custom|DropDownBox))
  (EventDispatchers|BindEventtoOnCheckStateChanged (Variables|/Game/UIClara/BP/Widget/Widget_Setting.Widget_Setting_C|GetToggleButton (Variables|Default|GetSettingWidget)) (delegate Custom|ToggleButton))
  (EventDispatchers|BindEventtoOnCheckStateChanged (Variables|/Game/UIClara/BP/Widget/Widget_Setting.Widget_Setting_C|GetCheckBox1 (Variables|Default|GetSettingWidget)) (delegate Custom|CheckBox1))
  (EventDispatchers|BindEventtoOnCheckStateChanged (Variables|/Game/UIClara/BP/Widget/Widget_Setting.Widget_Setting_C|GetCheckBox2 (Variables|Default|GetSettingWidget)) (delegate Custom|CheckBox2))
  (EventDispatchers|BindEventtoOnCheckStateChanged (Variables|/Game/UIClara/BP/Widget/Widget_Setting.Widget_Setting_C|GetCheckBox3 (Variables|Default|GetSettingWidget)) (delegate Custom|CheckBox3)))

(event OnComponentEndOverlap(Sphere)
  (params (OverlappedComponent :type Primitive%20Component%20Object%20Reference) (OtherActor :type Actor%20Object%20Reference) (OtherComp :type Primitive%20Component%20Object%20Reference) (OtherBodyIndex :type Integer))
  ;[1 1 1] Overlab Event for Adding Widget to Viewport
  (bind _asbp_character (Utilities|Casting|CastToBP_Character OtherActor))
  (Default|SettingUICancel _asbp_character))

(event Custom|SlideBar
  (params (Value :type Float%20%28single-precision%29))
  ;[1 1 1] Bind Setting UI Component Event
  (Transformation|SetRelativeScale3D (Variables|Default|GetSkeletalMesh) (Math|Conversions|ToVector(Float) (Math|Float|MapRangeClamped (Class|Slider|GetValue (Variables|/Game/UIClara/BP/Widget/Widget_Setting.Widget_Setting_C|GetSliderBar (Variables|Default|GetSettingWidget))) 0.0 1.0 0.5 2.0))))

(event Custom|RadioButton1
  (params (bIsChecked :type Boolean))
  (bind _settingwidget (Variables|Default|GetSettingWidget))
  ;[1 1 1] Bind Setting UI Component Event
  (if bIsChecked
    (Class|CheckBox|SetCheckedState (Variables|/Game/UIClara/BP/Widget/Widget_Setting.Widget_Setting_C|GetRadioButton1 _settingwidget) "Checked")
    (Class|CheckBox|SetCheckedState (Variables|/Game/UIClara/BP/Widget/Widget_Setting.Widget_Setting_C|GetRadioButton2 _settingwidget) "Unchecked")
    (Rendering|Material|SetVectorParameterValue (Variables|Default|GetUE4Man) "BodyColor" "(R=0.927083,G=0.087273,B=0.000000,A=1.000000)" :!class /Script/Engine.MaterialInstanceDynamic)))

(event Custom|RadioButton2
  (params (bIsChecked :type Boolean))
  (bind _settingwidget (Variables|Default|GetSettingWidget))
  ;[1 1 1] Bind Setting UI Component Event
  (if bIsChecked
    (Class|CheckBox|SetCheckedState (Variables|/Game/UIClara/BP/Widget/Widget_Setting.Widget_Setting_C|GetRadioButton2 _settingwidget) "Checked")
    (Class|CheckBox|SetCheckedState (Variables|/Game/UIClara/BP/Widget/Widget_Setting.Widget_Setting_C|GetRadioButton1 _settingwidget) "Unchecked")
    (Rendering|Material|SetVectorParameterValue (Variables|Default|GetUE4Man) "BodyColor" "(R=0.000000,G=0.139653,B=1.000000,A=1.000000)" :!class /Script/Engine.MaterialInstanceDynamic)))

(event Custom|DropDownBox
  (params (SelectedItem :type String) (SelectionType :type ESelectInfo%20Enum :default "OnKeyPress"))
  (bind _skeletalmesh (Variables|Default|GetSkeletalMesh))
  ;[1 1 1] Bind Setting UI Component Event
  (switch string (Class|ComboBoxString|GetSelectedOption (Variables|/Game/UIClara/BP/Widget/Widget_Setting.Widget_Setting_C|GetDropDownBox (Variables|Default|GetSettingWidget)))
    (:Idle
      (Components|Animation|PlayAnimation _skeletalmesh "/Game/UIClara/ThirdPerson/Mannequin/Animations/ThirdPersonIdle.ThirdPersonIdle" true))
    (:Walk
      (Components|Animation|PlayAnimation _skeletalmesh "/Game/UIClara/ThirdPerson/Mannequin/Animations/ThirdPersonWalk.ThirdPersonWalk" true))
    (:Run
      (Components|Animation|PlayAnimation _skeletalmesh "/Game/UIClara/ThirdPerson/Mannequin/Animations/ThirdPersonRun.ThirdPersonRun" true))))

(event Custom|ToggleButton
  (params (bIsChecked :type Boolean))
  (bind _ue4man (Variables|Default|GetUE4Man))
  ;[1 1 1] Bind Setting UI Component Event
  (if bIsChecked
    (Rendering|Material|SetScalarParameterValue _ue4man "Emissive" 5e+01 :!class /Script/Engine.MaterialInstanceDynamic)
    (else
      (Rendering|Material|SetScalarParameterValue _ue4man "Emissive" 1.0 :!class /Script/Engine.MaterialInstanceDynamic))))

(event Custom|CheckBox1
  (params (bIsChecked :type Boolean))
  (bind _skeletalmesh (Variables|Default|GetSkeletalMesh))
  ;[1 1 1] Bind Setting UI Component Event
  (if bIsChecked
    (Rendering|SetVisibility _skeletalmesh true false)
    (else
      (Rendering|SetVisibility _skeletalmesh false false))))

(event Custom|CheckBox2
  (params (bIsChecked :type Boolean))
  (bind _skeletalmesh2 (Variables|Default|GetSkeletalMesh2))
  ;[1 1 1] Bind Setting UI Component Event
  (if bIsChecked
    (Rendering|SetVisibility _skeletalmesh2 true false)
    (else
      (Rendering|SetVisibility _skeletalmesh2 false false))))

(event Custom|CheckBox3
  (params (bIsChecked :type Boolean))
  (bind _skeletalmesh3 (Variables|Default|GetSkeletalMesh3))
  ;[1 1 1] Bind Setting UI Component Event
  (if bIsChecked
    (Rendering|SetVisibility _skeletalmesh3 true false)
    (else
      (Rendering|SetVisibility _skeletalmesh3 false false))))

(event EventBeginPlay
  (bind _skeletalmesh (Variables|Default|GetSkeletalMesh))
  ;[1 1 1] Description Widget
  (bind _returnvalue (UserInterface|CreateWidget "/Game/UIClara/BP/Widget/WBP_DescriptionPanel.WBP_DescriptionPanel_C"))
  (bind _output_get (Variables|Default|SetDescriptionPanelWidget _returnvalue))
  (UserInterface|SetWidget (Variables|Default|GetDescriptionWidget) _output_get)
  (Rendering|Components|TextRender|SetText (Variables|/Game/UIClara/BP/Widget/WBP_DescriptionPanel.WBP_DescriptionPanel_C|GetTitleText (Variables|Default|GetDescriptionPanelWidget)) (Utilities|Text|ToText(String) "Setting"))
  (Rendering|Components|TextRender|SetText (Variables|/Game/UIClara/BP/Widget/WBP_DescriptionPanel.WBP_DescriptionPanel_C|GetDescriptionText (Variables|Default|GetDescriptionPanelWidget)) (Utilities|Text|ToText(String) (Utilities|String|Append "1) Blueprint : BP_Setting" " 
" "2) Widget : Widget_Setting" " 
" "4) Image : IMG_RadioButton_Checked, IMG_RadioButton_Unchecked, 
IMG_ToggleButton_On, IMG_ToggleButton_Off, IMG_CheckBox_Check, 
IMG_CheckBox_Uncheck, IMG_Button1_Normal, IMG_Button1_Hover, 
IMG_Button1_Pressed, IMG_Button1_Disabled, IMG_SortingBack")))
  (bind _returnvalue_2 (Rendering|Material|CreateDynamicMaterialInstance "/Game/UIClara/Sources/Material/MI_Character.MI_Character" "None" :!class /Script/Engine.KismetMaterialLibrary))
  (Variables|Default|SetUE4Man _returnvalue_2)
  (Rendering|Material|SetMaterial _skeletalmesh 0 (Variables|Default|GetUE4Man))
  (Rendering|Material|SetMaterial _skeletalmesh 1 (Variables|Default|GetUE4Man))
  (Rendering|Material|SetVectorParameterValue (Variables|Default|GetUE4Man) "BodyColor" "(R=0.927083,G=0.087273,B=0.000000,A=1.000000)" :!class /Script/Engine.MaterialInstanceDynamic))

(fn ConstructionScript)