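; BP_3DGUI is an example actor showing a layered 3D circular HUD with a live clock and a description panel.
; BeginPlay creates the widgets, sharing three circle-HUD instances across nine widget components.
; BP_Character overlapping the sphere plays sounds, neon and clock animations, and a timeline offsetting layers in depth by different factors; leaving reverses them.
; While active, Tick rolls the rings at varied speeds and updates the zero-padded system time.
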(event OnComponentBeginOverlap(Sphere)
  (params (OverlappedComponent :type Primitive%20Component%20Object%20Reference) (OtherActor :type Actor%20Object%20Reference) (OtherComp :type Primitive%20Component%20Object%20Reference) (OtherBodyIndex :type Integer) (bFromSweep :type Boolean) (SweepResult :type Hit%20Result%20Structure%20%28by%20ref%29))
  (bind _clockwidget (Variables|Default|GetClockWidget))
  (bind _circlehud4 (Variables|Default|GetCircleHUD4))
  (bind _circlehud1 (Variables|Default|GetCircleHUD1))
  (bind _circlehud3 (Variables|Default|GetCircleHUD3))
  ;[1 1 1] Overlab Event for Adding Widget to Viewport
  (Utilities|Casting|CastToBP_Character OtherActor)
  (Variables|Default|SetHUDOn true)
  ;[1 1 1] Clock_Opacity Animation
  (UserInterface|Animation|PlayAnimation _clockwidget (Variables|/Game/UIClara/BP/Widget/WBP_Clock.WBP_Clock_C|GetVisibilityAnim _clockwidget) 0.0 1 "Forward" 1.0)
  ;[1 1 1] Circle HUD_Neon On Animation
  (Audio|PlaySound2D "/Game/UIClara/Sources/Music/S_Clock_Cue.S_Clock_Cue" 1.0 1.0 0.0 0 0)
  (Utilities|FlowControl|Sequence
    (:then_0
      (UserInterface|Animation|PlayAnimation _circlehud4 (Variables|/Game/UIClara/BP/Widget/WBP_CircleHUD4.WBP_CircleHUD4_C|GetNeonOn _circlehud4) 0.0 1 "Forward" 1.0)
      ;[1 1 1] Circle HUD_Depth Animation
      (bind _newtrack_0 (Timeline|Timeline_0 Play)
        (:Update
          (Utilities|FlowControl|Sequence
            (:then_0
              (Transformation|SetRelativeLocation (Variables|Default|GetWidget7) (Math|Vector|MakeVector (* _newtrack_0 0.6) 0.0 1.8e+02) false false))
            (:then_1
              (Transformation|SetRelativeLocation (Variables|Default|GetWidget3) (Math|Vector|MakeVector (* _newtrack_0 0.9) 0.0 1.8e+02) false false)
              (Transformation|SetRelativeLocation (Variables|Default|GetWidget6) (Math|Vector|MakeVector (* _newtrack_0 0.85) 0.0 1.8e+02) false false))
            (:then_2
              (Transformation|SetRelativeLocation (Variables|Default|GetWidget4) (Math|Vector|MakeVector (* _newtrack_0 0.4) 0.0 1.8e+02) false false)
              (Transformation|SetRelativeLocation (Variables|Default|GetWidget8) (Math|Vector|MakeVector (* _newtrack_0 1.3) 0.0 1.8e+02) false false))
            (:then_3
              (Transformation|SetRelativeLocation (Variables|Default|GetWidget2) (Math|Vector|MakeVector (* _newtrack_0 0.3) 0.0 1.8e+02) false false)
              (Transformation|SetRelativeLocation (Variables|Default|GetWidget9) (Math|Vector|MakeVector (* _newtrack_0 1.6) 0.0 1.8e+02) false false))
            (:then_4
              (Transformation|SetRelativeLocation (Variables|Default|GetWidget5) (Math|Vector|MakeVector (* _newtrack_0 0.2) 0.0 1.8e+02) false false))))
        (:Finished
          (Audio|PlaySound2D "/Game/UIClara/Sources/Music/S_HoveredSound_Cue2.S_HoveredSound_Cue2" 1.0 1.0 0.0 0 0))))
    (:then_1
      (UserInterface|Animation|PlayAnimation _circlehud1 (Variables|/Game/UIClara/BP/Widget/WBP_CircleHUD.WBP_CircleHUD_C|GetNeonOn _circlehud1) 0.0 1 "Forward" 1.0))
    (:then_2
      (UserInterface|Animation|PlayAnimation _circlehud3 (Variables|/Game/UIClara/BP/Widget/WBP_CircleHUD3.WBP_CircleHUD3_C|GetNeonOn _circlehud3) 0.0 1 "Forward" 1.0))))

(event OnComponentEndOverlap(Sphere)
  (params (OverlappedComponent :type Primitive%20Component%20Object%20Reference) (OtherActor :type Actor%20Object%20Reference) (OtherComp :type Primitive%20Component%20Object%20Reference) (OtherBodyIndex :type Integer))
  (bind _clockwidget (Variables|Default|GetClockWidget))
  (bind _circlehud4 (Variables|Default|GetCircleHUD4))
  (bind _circlehud1 (Variables|Default|GetCircleHUD1))
  (bind _circlehud3 (Variables|Default|GetCircleHUD3))
  ;[1 1 1] Overlab Event for Adding Widget to Viewport
  (Utilities|Casting|CastToBP_Character OtherActor)
  (Variables|Default|SetHUDOn false)
  ;[1 1 1] Clock_Opacity Animation
  (UserInterface|Animation|PlayAnimation _clockwidget (Variables|/Game/UIClara/BP/Widget/WBP_Clock.WBP_Clock_C|GetVisibilityAnim _clockwidget) 0.0 1 "Reverse" 1.0)
  ;[1 1 1] Circle HUD_Neon On Animation
  (Audio|PlaySound2D "/Game/UIClara/Sources/Music/S_Clock_Cue.S_Clock_Cue" 1.0 1.0 0.0 0 0)
  (Utilities|FlowControl|Sequence
    (:then_0
      (UserInterface|Animation|PlayAnimation _circlehud4 (Variables|/Game/UIClara/BP/Widget/WBP_CircleHUD4.WBP_CircleHUD4_C|GetNeonOn _circlehud4) 0.0 1 "Reverse" 1.0)
      ;[1 1 1] Circle HUD_Depth Animation
      (bind _newtrack_0 (Timeline|Timeline_0 ReverseFromEnd)
        (:Update
          (Utilities|FlowControl|Sequence
            (:then_0
              (Transformation|SetRelativeLocation (Variables|Default|GetWidget7) (Math|Vector|MakeVector (* _newtrack_0 0.6) 0.0 1.8e+02) false false))
            (:then_1
              (Transformation|SetRelativeLocation (Variables|Default|GetWidget3) (Math|Vector|MakeVector (* _newtrack_0 0.9) 0.0 1.8e+02) false false)
              (Transformation|SetRelativeLocation (Variables|Default|GetWidget6) (Math|Vector|MakeVector (* _newtrack_0 0.85) 0.0 1.8e+02) false false))
            (:then_2
              (Transformation|SetRelativeLocation (Variables|Default|GetWidget4) (Math|Vector|MakeVector (* _newtrack_0 0.4) 0.0 1.8e+02) false false)
              (Transformation|SetRelativeLocation (Variables|Default|GetWidget8) (Math|Vector|MakeVector (* _newtrack_0 1.3) 0.0 1.8e+02) false false))
            (:then_3
              (Transformation|SetRelativeLocation (Variables|Default|GetWidget2) (Math|Vector|MakeVector (* _newtrack_0 0.3) 0.0 1.8e+02) false false)
              (Transformation|SetRelativeLocation (Variables|Default|GetWidget9) (Math|Vector|MakeVector (* _newtrack_0 1.6) 0.0 1.8e+02) false false))
            (:then_4
              (Transformation|SetRelativeLocation (Variables|Default|GetWidget5) (Math|Vector|MakeVector (* _newtrack_0 0.2) 0.0 1.8e+02) false false))))
        (:Finished
          (Audio|PlaySound2D "/Game/UIClara/Sources/Music/S_HoveredSound_Cue2.S_HoveredSound_Cue2" 1.0 1.0 0.0 0 0))))
    (:then_1
      (UserInterface|Animation|PlayAnimation _circlehud1 (Variables|/Game/UIClara/BP/Widget/WBP_CircleHUD.WBP_CircleHUD_C|GetNeonOn _circlehud1) 0.0 1 "Reverse" 1.0))
    (:then_2
      (UserInterface|Animation|PlayAnimation _circlehud3 (Variables|/Game/UIClara/BP/Widget/WBP_CircleHUD3.WBP_CircleHUD3_C|GetNeonOn _circlehud3) 0.0 1 "Reverse" 1.0))))

(event EventBeginPlay
  ;[1 1 1] Description Widget
  (bind _returnvalue (UserInterface|CreateWidget "/Game/UIClara/BP/Widget/WBP_DescriptionPanel.WBP_DescriptionPanel_C"))
  (bind _output_get (Variables|Default|SetDescriptionPanelWidget _returnvalue))
  (UserInterface|SetWidget (Variables|Default|GetDescriptionWidget) _output_get)
  (Rendering|Components|TextRender|SetText (Variables|/Game/UIClara/BP/Widget/WBP_DescriptionPanel.WBP_DescriptionPanel_C|GetTitleText (Variables|Default|GetDescriptionPanelWidget)) (Utilities|Text|ToText(String) "3D GUI"))
  (Rendering|Components|TextRender|SetText (Variables|/Game/UIClara/BP/Widget/WBP_DescriptionPanel.WBP_DescriptionPanel_C|GetDescriptionText (Variables|Default|GetDescriptionPanelWidget)) (Utilities|Text|ToText(String) (Utilities|String|Append "1) Blueprint : BP_3DGUI" " 
" "2) WidgetElement : WBP_CircleHUD, WBP_CircleHUD3, 
WBP_CircleHUD4, WBP_Clock" " 
" "3) Image : IMG_CircleHUD, IMG_CircleHUD3, 
IMG_CircleHUD4, IMG_CircleHUD_Neon, IMG_CircleHUD3_Neon, 
IMG_CircleHUD4_Neon")))
  (bind _returnvalue_2 (UserInterface|CreateWidget "/Game/UIClara/BP/Widget/WBP_Clock.WBP_Clock_C"))
  (bind _output_get_2 (Variables|Default|SetClockWidget _returnvalue_2))
  (UserInterface|SetWidget (Variables|Default|GetClock) _output_get_2)
  ;[1 1 1] Set 3D Widget
  (bind _returnvalue_3 (UserInterface|CreateWidget "/Game/UIClara/BP/Widget/WBP_CircleHUD.WBP_CircleHUD_C"))
  (bind _output_get_3 (Variables|Default|SetCircleHUD1 _returnvalue_3))
  (UserInterface|SetWidget (Variables|Default|GetWidget) _output_get_3)
  (bind _returnvalue_4 (UserInterface|CreateWidget "/Game/UIClara/BP/Widget/WBP_CircleHUD3.WBP_CircleHUD3_C"))
  (bind _output_get_4 (Variables|Default|SetCircleHUD3 _returnvalue_4))
  (UserInterface|SetWidget (Variables|Default|GetWidget2) _output_get_4)
  (bind _returnvalue_5 (UserInterface|CreateWidget "/Game/UIClara/BP/Widget/WBP_CircleHUD4.WBP_CircleHUD4_C"))
  (bind _output_get_5 (Variables|Default|SetCircleHUD4 _returnvalue_5))
  (UserInterface|SetWidget (Variables|Default|GetWidget3) _output_get_5))

(event EventTick
  (params (DeltaSeconds :type Float%20%28single-precision%29))
  (bind _returnvalue (Math|DateTime|Now))
  (bind _returnvalue_2 (Class|KismetMathLibrary|GetHour _returnvalue))
  (bind _returnvalue_3 (Class|KismetMathLibrary|GetMinute _returnvalue))
  (bind _returnvalue_4 (Class|KismetMathLibrary|GetSecond _returnvalue))
  (if (Variables|Default|GetHUDOn)
    ;[1 1 1] Circle HUD_Rotate Animation
    (Transformation|AddRelativeRotation (Variables|Default|GetWidget3) (Math|Rotator|MakeRotator (* DeltaSeconds 15.0) 0.0 0.0) false false)
    (Transformation|AddRelativeRotation (Variables|Default|GetWidget2) (Math|Rotator|MakeRotator (* DeltaSeconds 25.0) 0.0 0.0) false false)
    (Transformation|AddRelativeRotation (Variables|Default|GetWidget4) (Math|Rotator|MakeRotator (* DeltaSeconds 3e+01) 0.0 0.0) false false)
    (Utilities|FlowControl|Sequence
      (:then_0
        ;[1 1 1] Set Time Text
        (if (< (/ _returnvalue_2 10) 1)
          (Variables|Default|SetHour (Utilities|String|Append "0" (Utilities|String|ToString(Integer) _returnvalue_2)))
          (else
            (Variables|Default|SetHour (Utilities|String|ToString(Integer) _returnvalue_2)))))
      (:then_1
        (if (< (/ _returnvalue_3 10) 1)
          (Variables|Default|SetMin (Utilities|String|Append "0" (Utilities|String|ToString(Integer) _returnvalue_3)))
          (else
            (Variables|Default|SetMin (Utilities|String|ToString(Integer) _returnvalue_3)))))
      (:then_2
        (if (< (/ _returnvalue_4 10) 1)
          (Variables|Default|SetSec (Utilities|String|Append "0" (Utilities|String|ToString(Integer) _returnvalue_4)))
          (else
            (Variables|Default|SetSec (Utilities|String|ToString(Integer) _returnvalue_4)))))
      (:then_3
        (Rendering|Components|TextRender|SetText (Variables|/Game/UIClara/BP/Widget/WBP_Clock.WBP_Clock_C|GetTextBlock_0 (Variables|Default|GetClockWidget)) (Utilities|Text|ToText(String) (Utilities|String|Append (Variables|Default|GetHour) ":" (Variables|Default|GetMin) ":" (Variables|Default|GetSec))))))))

(fn ConstructionScript)