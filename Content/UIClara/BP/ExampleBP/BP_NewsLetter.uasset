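; BP_NewsLetter is an example actor that demonstrates a newsletter UI when the player character walks up to it.
; On BeginPlay it creates a WBP_DescriptionPanel for its DescriptionWidget component, titled and filled with the names of the blueprint, widget and images used.
; Sphere begin and end overlaps cast to BP_Character and call NewsLetter or NewsLetterCancel, leaving the newsletter display logic to the character.
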(event OnComponentBeginOverlap(Sphere)
  (params (OverlappedComponent :type Primitive%20Component%20Object%20Reference) (OtherActor :type Actor%20Object%20Reference) (OtherComp :type Primitive%20Component%20Object%20Reference) (OtherBodyIndex :type Integer) (bFromSweep :type Boolean) (SweepResult :type Hit%20Result%20Structure%20%28by%20ref%29))
  ;[1 1 1] Overlab Event for Adding Widget to Viewport
  (bind _asbp_character (Utilities|Casting|CastToBP_Character OtherActor))
  (Default|NewsLetter _asbp_character))

(event OnComponentEndOverlap(Sphere)
  (params (OverlappedComponent :type Primitive%20Component%20Object%20Reference) (OtherActor :type Actor%20Object%20Reference) (OtherComp :type Primitive%20Component%20Object%20Reference) (OtherBodyIndex :type Integer))
  ;[1 1 1] Overlab Event for Adding Widget to Viewport
  (bind _asbp_character (Utilities|Casting|CastToBP_Character OtherActor))
  (Default|NewsLetterCancel _asbp_character))

(event EventBeginPlay
  ;[1 1 1] Description Widget
  (bind _returnvalue (UserInterface|CreateWidget "/Game/UIClara/BP/Widget/WBP_DescriptionPanel.WBP_DescriptionPanel_C"))
  (bind _output_get (Variables|Default|SetDescriptionPanelWidget _returnvalue))
  (UserInterface|SetWidget (Variables|Default|GetDescriptionWidget) _output_get)
  (Rendering|Components|TextRender|SetText (Variables|/Game/UIClara/BP/Widget/WBP_DescriptionPanel.WBP_DescriptionPanel_C|GetTitleText (Variables|Default|GetDescriptionPanelWidget)) (Utilities|Text|ToText(String) "NewsLetter"))
  (Rendering|Components|TextRender|SetText (Variables|/Game/UIClara/BP/Widget/WBP_DescriptionPanel.WBP_DescriptionPanel_C|GetDescriptionText (Variables|Default|GetDescriptionPanelWidget)) (Utilities|Text|ToText(String) (Utilities|String|Append "1) Blueprint : BP_NewsLetter" " 
" "2) Widget : Widget_NewsLetter" " 
" "3) Image : IMG_Icon_letter, IMG_Popup, 
IMG_Button1_Normal, IMG_Button1_Hover, 
IMG_Button1_Pressed"))))

(fn ConstructionScript)